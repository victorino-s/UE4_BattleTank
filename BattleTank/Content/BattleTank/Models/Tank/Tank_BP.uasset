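; Tank pawn Blueprint that handles player camera aiming for the battle tank.
; The AimAzimuth axis yaws an AzimuthGimbal component and AimAltitude pitches the SpringArm, separating horizontal and vertical orbit.
; Each axis is scaled by its own sensitivity, and BeginPlay negates the vertical one when InvertY is set.
; Tick, overlap and construction script are empty.
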(event `self.ReceiveBeginPlay`
  (if (`self.InvertY`)
    (set `self.YSensitivity` (* (`self.YSensitivity`) -1.0))))

(event `InputAxis|AimAzimuth`
  (params (AxisValue :type "Float (single-precision)"))
  ;[1 1 1] Camera Input Binding
  (`SceneComponent.K2_AddLocalRotation` (`self.Azimuth Gimbal`) (`KismetMathLibrary.MakeRotator` 0.0 0.0 (* AxisValue (`self.XSensitivity`))) false false))

(event `InputAxis|AimAltitude`
  (params (AxisValue :type "Float (single-precision)"))
  ;[1 1 1] Camera Input Binding
  (`SceneComponent.K2_AddLocalRotation` (`self.SpringArm`) (`KismetMathLibrary.MakeRotator` 0.0 (* AxisValue (`self.YSensitivity`))) false false))

(fn `UserConstructionScript`)